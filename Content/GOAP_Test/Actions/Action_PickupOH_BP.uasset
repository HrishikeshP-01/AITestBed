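; GOAP action that makes the AI character pick up an item and hold it in its right hand.
; Execute casts the blackboard's SelfActor to Character, snaps the item to its named socket and stores it in the Item_RH key.
; CalculateCurrentWS reports the equipped world state whenever Item_RH holds any valid object, without checking that it is this item.
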(event EventExecute
  (bind _item (Variables|Default|Getitem))
  (bind _ascharacter (Utilities|Casting|CastToCharacter (AI|Components|Blackboard|GetValueasObject (Variables|Default|Getbbc) (Utilities|Name|MakeLiteralName "SelfActor"))))
  (Transformation|AttachActorToActor _item _ascharacter (Variables|/Script/GOAP.Item|GetSocketName _item) "SnapToTarget" "SnapToTarget" "KeepRelative" true)
  ;[1 0.2031 0.2031] Simple implementation that assigns item to RH only
  (AI|Components|Blackboard|SetValueasObject (Variables|Default|Getbbc) (Utilities|Name|MakeLiteralName "Item_RH") (Variables|Default|Getitem)))

(fn CalculateCurrentWS
  ;[1 0.1406 0.1406] assuming the iobject in RH is the item!!!
  (Utilities|IsValid (AI|Components|Blackboard|GetValueasObject (Variables|Default|Getbbc) (Utilities|Name|MakeLiteralName "Item_RH"))
    (:Is%20Valid
      (return "Item_Equipped"))
    (:Is%20Not%20Valid
      (return "Item_Unequipped"))))