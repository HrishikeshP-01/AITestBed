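; GOAP action Blueprint that moves the owning actor toward its target, in what appears to be a GOAP test setup.
; Execute reads SelfActor and Target from the blackboard, prints both locations, then sets the actor's location directly to the MoveToPos result, without sweep.
; CalculateCurrentWS reports the world state as close-range or far proximity by comparing the distance between both actors to a fixed threshold.
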(event EventExecute
  (bind _asactor (Utilities|Casting|CastToActor (AI|Components|Blackboard|GetValueasObject (Variables|Default|Getbbc) (Utilities|Name|MakeLiteralName "SelfActor"))))
  (bind _asactor_2 (Utilities|Casting|CastToActor (AI|Components|Blackboard|GetValueasObject (Variables|Default|Getbbc) (Utilities|Name|MakeLiteralName "Target"))))
  (Development|PrintString (Utilities|String|ToString(Vector) (Transformation|GetActorLocation _asactor)))
  (Development|PrintString (Utilities|String|ToString(Vector) (Transformation|GetActorLocation _asactor_2)))
  (bind _returnvalue (Class|Moveto|MovetoPos (Transformation|GetActorLocation _asactor) (Transformation|GetActorLocation _asactor_2)))
  (Transformation|SetActorLocation _asactor _returnvalue false false))

(fn CalculateCurrentWS
  (bind _asactor (Utilities|Casting|CastToActor (AI|Components|Blackboard|GetValueasObject (Variables|Default|Getbbc) (Utilities|Name|MakeLiteralName "SelfActor"))))
  (bind _asactor_2 (Utilities|Casting|CastToActor (AI|Components|Blackboard|GetValueasObject (Variables|Default|Getbbc) (Utilities|Name|MakeLiteralName "Target"))))
  (if (< (Math|Vector|Distance(Vector) (Transformation|GetActorLocation _asactor) (Transformation|GetActorLocation _asactor_2)) 1e+02)
    (return "Proximity_CloseRange")
    (else
      (return "Proximity_Far"))))