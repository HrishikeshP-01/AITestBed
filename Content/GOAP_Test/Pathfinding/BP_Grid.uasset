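; BP_Grid is a pathfinding test actor that visualizes a grid and a path between its Start and End actors.
; The construction script draws or flushes the debug grid based on a DrawGrid toggle.
; BeginPlay redraws the grid, calls GetPath with both actor locations and marks each returned point with a debug sphere.
; Grid and path logic live outside these graphs; the line-segment drawing loops are disconnected.
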(event EventBeginPlay
  (Rendering|Debug|FlushPersistentDebugLines)
  (Variables|Temp|SetStartPt (Transformation|GetActorLocation (Variables|Temp|GetStart)))
  (Variables|Temp|SetEndPt (Transformation|GetActorLocation (Variables|Temp|GetEnd)))
  (Class|Grid|DrawGrid)
  (bind _path (Class|Grid|GetPath (Variables|Temp|GetStartPt) (Variables|Temp|GetEndPt)))
  (for _array_element _path
    (Rendering|Debug|DrawDebugSphere _array_element 3e+01 8 "(R=0.440000,G=0.000000,B=0.086819,A=1.000000)" 5e+01))
  (Development|PrintString "Hello"))

(event Collision|EventActorBeginOverlap
  (params (OtherActor :type Actor%20Object%20Reference)))

(event EventTick
  (params (DeltaSeconds :type Float%20%28single-precision%29)))

(fn ConstructionScript
  (if (Variables|Default|GetbDrawGrid)
    (Class|Grid|DrawGrid)
    (else
      (Rendering|Debug|FlushPersistentDebugLines))))